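; Base pickup actor with a physics-simulated skeletal mesh that signals players when they are within range.
; Sphere begin and end overlaps run only with authority and call SetPickupInfoMessage on actors tagged Player, passing the pickup and overlap state.
; DisablePhysics stops simulation and turns off collision on both mesh and sphere.
; Getters expose a fixed interact type and the pickup type stored in PickupInfo.
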(event `self.ReceiveBeginPlay`
  (`PrimitiveComponent.SetSimulatePhysics` (`self.SkeletalMesh`) true))

(event `/Game/_Main/Interfaces/INT_Pickups.DisablePhysics`
  (bind _skeletalmesh (`self.SkeletalMesh`))
  (`PrimitiveComponent.SetSimulatePhysics` _skeletalmesh false)
  (`PrimitiveComponent.SetCollisionEnabled` _skeletalmesh "NoCollision")
  (`PrimitiveComponent.SetCollisionEnabled` (`self.Sphere`) "NoCollision"))

(event `self.Sphere.OnComponentBeginOverlap`
  (params (OverlappedComponent :type "PrimitiveComponent Object Reference") (OtherActor :type "Actor Object Reference") (OtherComp :type "PrimitiveComponent Object Reference") (OtherBodyIndex :type Integer) (bFromSweep :type Boolean) (SweepResult :type "HitResult Structure (by ref)"))
  (`/Engine/EditorBlueprintResources/ActorMacros.Switch Has Authority`
    (:`Authority`
      (if (`self.ActorHasTag` OtherActor "Player")
        (message `/Game/_Main/Interfaces/INT_BunkerPlayerCharacter.SetPickupInfo` OtherActor self true)))))

(event `self.Sphere.OnComponentEndOverlap`
  (params (OverlappedComponent :type "PrimitiveComponent Object Reference") (OtherActor :type "Actor Object Reference") (OtherComp :type "PrimitiveComponent Object Reference") (OtherBodyIndex :type Integer))
  (`/Engine/EditorBlueprintResources/ActorMacros.Switch Has Authority`
    (:`Authority`
      (if (`self.ActorHasTag` OtherActor "Player")
        (message `/Game/_Main/Interfaces/INT_BunkerPlayerCharacter.SetPickupInfo` OtherActor self false)))))

(fn `GetInteractType`
  (returns (InteractType :type "/Game/_Main/BaseClasses/E_InteractType Enum"))
  (return "NewEnumerator0"))

(fn `GetPickupType`
  (returns (PickupType :type "/Game/_Main/Pickups/E_PickupTypes Enum"))
  (return (`.PickupType_20_8FAF3773487EF5AA1EED3AB38FAA0FD7` (break `/Game/_Main/Pickups/S_PickupInfo` (`self.PickupInfo`)))))

(fn `UserConstructionScript`
  (`parent.UserConstructionScript`))