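; Player controller for the bunker character that owns the local player's main HUD and weapon widgets.
; After a short delay on BeginPlay, it creates both widgets and adds them to the viewport, for local controllers only.
; Its events forward pickup-name messages and stamina updates to the main widget, and visibility state to the weapon widget.
; CreateMainWidget and CreateWeaponWidget are empty stubs, though ShowWeaponWidgets still calls the former.
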(event `CreateWeaponWidget`)

(event `CreateMainWidget`)

(event `self.ReceiveBeginPlay`
  (`KismetSystemLibrary.Delay` 0.2)
  (if (`self.IsLocalPlayerController`)
    (bind _returnvalue (`|CreateWidget` "/Game/_Main/Widgets/MainWidget_W.MainWidget_W_C"))
    (bind _output_get (set `self.PlayerUI` _returnvalue))
    (`UserWidget.AddToViewport` _output_get 0)
    (bind _returnvalue_2 (`|CreateWidget` "/Game/_Main/Widgets/WeaponWidget.WeaponWidget_C"))
    (bind _output_get_2 (set `self.PlayerWeaponWidgetUI` _returnvalue_2))
    (`UserWidget.AddToViewport` _output_get_2 0)))

(event `/Game/_Main/Interfaces/INT_BunkerCharacterController.ShowPickupName`
  (params (State :type Boolean) (Name :type Text))
  (`/Game/_Main/Widgets/MainWidget_W.PlayerMessage` (`self.PlayerUI`) State Name))

(event `/Game/_Main/Interfaces/INT_BunkerCharacterController.ShowWeaponWidgets`
  (params (State :type Boolean))
  (`self.CreateMainWidget`)
  (`/Game/_Main/Widgets/WeaponWidget.WeaponWidgetsDisplay` (`self.PlayerWeaponWidgetUI`) State))

(event `/Game/_Main/Interfaces/INT_BunkerCharacterController.UpdateStaminaUI`
  (params (Stamina :type "Float (double-precision)"))
  (`/Game/_Main/Widgets/MainWidget_W.UpdateStaminaBar` (`self.PlayerUI`) Stamina))

(fn `UserConstructionScript`)