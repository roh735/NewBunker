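; Base enemy Blueprint that takes weapon hits, tracks health and ragdolls on death.
; EnemyTakeDamage scales weapon damage by the hit physical material's DestructibleDamageThresholdScale, giving per-surface multipliers, then subtracts it from health.
; Non-lethal hits print the damage.
; Death enables mesh physics, plays a sound, applies the player's Beretta kill impulse away from the player on the hit bone, and destroys the capsule.
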(event `self.ReceiveBeginPlay`
  (bind _asbp_first_person_character (cast `/Game/_Main/Blueprints/Character/BP_FirstPersonCharacter` (`GameplayStatics.GetPlayerCharacter` 0)))
  (set `self.Player` _asbp_first_person_character))

(event `/Game/_Main/InterfacesTest/BPITakeDamage.EnemyTakeDamage`
  (params (WeaponStats :type "/Game/_Main/Data/S_WeaponStats Structure") (HitResult :type "HitResult Structure"))
  (bind (_bblockinghit _binitialoverlap _time _distance _location _impactpoint _normal _impactnormal _physmat _hitactor _hitcomponent _hitbonename) (`GameplayStatics.BreakHitResult` HitResult))
  (if (not (`self.isDead?`))
    (bind _calculateddamage (`self.calculateDamage` (`.Damage_3_04590C9048D57529BF7018B81CD7FB62` (break `/Game/_Main/Data/S_WeaponStats` WeaponStats)) HitResult))
    (bind _isdead (`self.healthUpdate` _calculateddamage))
    (bind _output_get (set `self.isDead?` _isdead))
    (if _output_get
      (`self.EnemyDeath` _impactnormal _hitbonename)
      (else
        (`KismetSystemLibrary.PrintString` (`KismetStringLibrary.Conv_DoubleToString` _calculateddamage))))))

(fn `calculateDamage`
  (params (Damage :type "Float (double-precision)") (HitResult :type "HitResult Structure"))
  (returns (CalculatedDamage :type "Float (double-precision)"))
  (locals (LocalDamage :type "Float (double-precision)"))
  (set `local.LocalDamage` Damage)
  (return (* (`local.LocalDamage`) (`PhysicalMaterial.DestructibleDamageThresholdScale` (`.PhysMat` (`GameplayStatics.BreakHitResult` HitResult))))))

(fn `EnemyDeath`
  (params (HitLocation :type "Vector Structure") (boneName :type Name))
  (bind _player (`self.Player`))
  (`|ExecutionSequence`
    (:`then_0`
      ;[1 0 0] Enabling ragdoll physics
      (`PrimitiveComponent.SetSimulatePhysics` (`self.Mesh`) true))
    (:`then_1`
      (`GameplayStatics.PlaySound2D` null 1.0 1.0 0.0 null null))
    (:`then_2`
      (`PrimitiveComponent.AddImpulseAtLocation` (`self.Mesh`) (* (`KismetMathLibrary.GetDirectionUnitVector` (`self.K2_GetActorLocation` _player) (`self.K2_GetActorLocation`)) (`/Game/_Main/Pickups/Beretta/Beretta.KillImpuls` (cast `/Game/_Main/Pickups/Beretta/Beretta` (`/Game/_Main/Blueprints/Character/BP_FirstPersonCharacter.MyCurrentWeapon` _player) :!pure true))) HitLocation boneName)
      (`ActorComponent.K2_DestroyComponent` (`self.CapsuleComponent`)))))

(fn `healthUpdate`
  (params (DamageApplied :type "Float (double-precision)"))
  (returns (isDead :type Boolean))
  (locals (`LocalIsDead?` :type Boolean))
  (`|ExecutionSequence`
    (:`then_0`
      (if (>= DamageApplied (`self.CurrentHealth`))
        (set `local.LocalIsDead?` true)
        (set `self.CurrentHealth` 0.0)
        (else
          (set `self.CurrentHealth` (- (`self.CurrentHealth`) DamageApplied)))))
    (:`then_1`
      (return (`local.LocalIsDead?`)))))

(fn `UserConstructionScript`)