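; BP_RussianBase is an AI enemy character that chases the player and plays random attack montages.
; An AIMoveTo loop targets player controller 0, alternating movement and attacks until death, while sighting any pawn sets walk speed.
; Point damage lowers health and triggers Multi-prefixed events for blood, sound and hit montages.
; Death stops movement, applies ragdoll collision and plays a death animation; the detach and delayed-destroy cleanup is unwired.
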(event `self.ReceivePointDamage`
  (params (Damage :type "Float (single-precision)") (DamageType :type "DamageType Object Reference") (HitLocation :type "Vector Structure") (HitNormal :type "Vector Structure") (HitComponent :type "PrimitiveComponent Object Reference") (BoneName :type Name) (ShotFromDirection :type "Vector Structure") (InstigatedBy :type "Controller Object Reference") (DamageCauser :type "Actor Object Reference") (HitInfo :type "HitResult Structure (by ref)"))
  ;[1 1 1] AI Accept Damage
  (if (not (`self.isDeath?`))
    (`self.Multi_AIHitGetDamageEffect` "/Game/_Main/AI/P_AI_Hit_Blood.P_AI_Hit_Blood" (`self.K2_GetActorLocation`) null (`KismetArrayLibrary.Array_Random` (`|MakeArray` (`self.HitAnimationMontageOne`) (`self.HitAnimationMontageTwo`))) DamageCauser Damage)
    (if (<= (`self.Health`) 0.0)
      (`self.Death`)
      (else
        (bind _output_get (set `self.Health` (- (`self.Health`) Damage)))
        (if (<= _output_get 0.0)
          (`self.Death`))))))

(event `Multi_AIHitGetDamageEffect`
  (params (EmitterTemplate :type "ParticleSystem Object Reference") (Location :type "Vector Structure") (Sound :type "SoundBase Object Reference") (MontageToPlay :type "AnimMontage Object Reference") (Target :type "Object Object Reference") (Damage :type "Float (double-precision)"))
  ;[1 1 1] Get damage efects
  (`GameplayStatics.SpawnEmitterAtLocation` EmitterTemplate Location)
  (`GameplayStatics.PlaySoundAtLocation` Sound Location (struct) 1.0 1.0 0.0 null null null null)
  (`|PlayMontage` (`self.Mesh`) MontageToPlay))

(event `self.PawnSensing.OnSeePawn`
  (params (Pawn :type "Pawn Object Reference"))
  (set `CharacterMovementComponent.MaxWalkSpeed` 360.0 (`self.CharacterMovement`)))

(event `self.ReceiveBeginPlay`
  (`self.RunToPlayer`))

(event `RunToPlayer`
  (if (not (`self.isDeath?`))
    (`|AIMoveTo` self (0.0 0.0 0.0) (`GameplayStatics.GetPlayerController` 0) 40.0
      (:`OnSuccess`
        (`self.AttackPlayer`))
      (:`OnFail`
        (`self.RunToPlayer`)))))

(event `Death`
  ;[1 1 1] AI Death Event
  (if (not (`self.isDeath?`))
    (set `self.isDeath?` true)
    (`MovementComponent.StopMovementImmediately` (`self.CharacterMovement`))
    (`self.Multi_DeadAnimation`)))

(event `AttackPlayer`
  (if (not (`self.isDeath?`))
    (`|PlayMontage` (`self.Mesh`) (`KismetArrayLibrary.Array_Random` (`|MakeArray` (`self.AttackAnimMontageOne`) (`self.AttackAnimMontageTwo`)))
      (:`OnCompleted`
        _)
      (:`OnInterrupted`
        _))
    (`self.RunToPlayer`)))

(event `Multi_DeadAnimation`
  ;[1 1 1] AI Death Event
  (`PrimitiveComponent.SetCollisionProfileName` (`self.CapsuleComponent`) "Ragdoll" true)
  (`PrimitiveComponent.SetCollisionProfileName` (`self.Mesh`) "Ragdoll" true)
  (`SkeletalMeshComponent.SetAnimationMode` (`self.Mesh`) "AnimationSingleNode")
  (`self.f_PlayDeathAnimation`))

(fn `f_PlayDeathAnimation`
  (`SkeletalMeshComponent.PlayAnimation` (`self.Mesh`) (`self.DeathAnimMontage`) false))

(fn `UserConstructionScript`)